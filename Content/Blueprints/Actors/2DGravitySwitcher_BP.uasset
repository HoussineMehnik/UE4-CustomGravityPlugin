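; 2DGravitySwitcher_BP is a placeable trigger actor that changes the gravity direction of a 2DCharacter_BP that overlaps it.
; The chosen 2DGravityDirection (Up, Down, Left or Right) maps to a world vector passed to the character's SetGravityDirection.
; A DoOnce gate with a three-second delayed reset throttles repeat triggering.
; The construction script rotates the shape plane to match the selected direction.
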(event EventActorBeginOverlap
  (params (OtherActor :type Actor%20Object%20Reference))
  (bind _as2dcharacter_bp (Utilities|Casting|CastTo2DCharacter_BP OtherActor))
  (Utilities|FlowControl|DoOnce false :!label _label
    (:Completed
      (Default|SetGravityDirection _as2dcharacter_bp (Utilities|Select :Index (Variables|Default|Get2DGravityDirection) :NewEnumerator0 "0,0,1.000000" :NewEnumerator1 "0,0,-1.000000" :NewEnumerator2 "1.000000,0,0" :NewEnumerator3 "-1.000000,0,0"))
      (Utilities|FlowControl|Delay 3.0)
      (goto _label Reset))))

(fn ConstructionScript
  (Transformation|SetRelativeRotation (Variables|Default|GetSM_Shape_Plane) (Math|Rotator|MakeRotator 9e+01 (Utilities|Select :Index (Variables|Default|Get2DGravityDirection) :NewEnumerator0 0.0 :NewEnumerator1 1.8e+02 :NewEnumerator2 -9e+01 :NewEnumerator3 9e+01) 0.0) false false))