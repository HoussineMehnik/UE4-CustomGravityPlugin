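; Player pawn for a 2D Paper2D side-view game with changeable gravity direction and a world-fixed camera boom.
; Each tick picks the idle, running or falling flipbook, rolls or pitches it to the actor's up vector and flips it toward travel.
; Input moves along world X or Z, whichever is perpendicular to up.
; SetGravityDirection applies new gravity and zeroes air control, which is restored upon grounding.
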(event Custom|UpdateFlipbookFacingDirection
  (bind _movementcomponent (Variables|Default|GetMovementComponent))
  (bind _returnvalue (Class|CustomMovementComponent|GetMovementVelocity _movementcomponent))
  (if (!= (.x _returnvalue) 0.0)
    (Transformation|SetRelativeScale3D (Variables|Default|GetCharacter_Flipbook) (Math|Vector|MakeVector (* (Math|Float|Sign(Float) (.x _returnvalue)) (Math|Float|Sign(Float) (Math|Vector|DotProduct (Transformation|GetActorUpVector) "0.000000,0.000000,1.000000"))) 1.0 1.0))))

(event Custom|Update%20Air%20Control%20Ratio
  (if (AI|Components|NavMovement|IsMovingonGround (Variables|Default|GetMovementComponent))
    (Utilities|FlowControl|DoOnce false :!label _label
      (:Completed
        (Variables|/Script/CustomGravityPlugin.CustomMovementComponent|SetAirControlRatio (Variables|Default|GetMovementComponent) 1.0)))
    (else
      (goto _label Reset))))

(event Custom|Update%20Animation
  (if (AI|Components|NavMovement|IsMovingonGround (Variables|Default|GetMovementComponent))
    (Sprite|SetFlipbook (Variables|Default|GetCharacter_Flipbook) (select (> (Class|CustomMovementComponent|GetCurrentWalkSpeed (Variables|Default|GetMovementComponent)) 5.0) "/Game/2DAssets/Character/Run/RunningFlipbook.RunningFlipbook" "/Game/2DAssets/Character/Idle/IdleFlipbook.IdleFlipbook"))
    (else
      (Sprite|SetFlipbook (Variables|Default|GetCharacter_Flipbook) (select (> (.z (Class|CustomMovementComponent|GetFallingVelocity (Variables|Default|GetMovementComponent))) 0.0) "/Game/2DAssets/Character/Fall/FallingFlipbook.FallingFlipbook" "/Game/2DAssets/Character/Fall/FallingFlipbook.FallingFlipbook")))))

(event Custom|SetGravityDirection
  (params (New%20Gravity%20Direction :type Vector))
  (Variables|/Script/CustomGravityPlugin.CustomMovementComponent|SetCustomGravityInfo (Variables|Default|GetMovementComponent) (Utilities|Struct|MakeGravityInfo 9.8e+02 New%20Gravity%20Direction "EFM_Acceleration" true))
  (Variables|/Script/CustomGravityPlugin.CustomMovementComponent|SetAirControlRatio (Variables|Default|GetMovementComponent) 0.0)
  (Utilities|FlowControl|Delay 0.05)
  (Class|CustomMovementComponent|RequestGavityImmediateUpdate (Variables|Default|GetMovementComponent)))

(event EventBeginPlay
  (Variables|/Script/Engine.SceneComponent|SetbAbsoluteRotation (Variables|Default|GetSpringArm) true)
  (Transformation|SetWorldRotation (Variables|Default|GetSpringArm) "0,-90.000000, 0" false false)
  (Variables|/Script/Engine.SceneComponent|SetbAbsoluteRotation (Variables|Default|GetFlipbook_ROOT) true))

(event EventActorBeginOverlap
  (params (OtherActor :type Actor%20Object%20Reference)))

(event EventTick
  (params (DeltaSeconds :type Float%20%28single-precision%29))
  (bind _returnvalue (Transformation|GetActorUpVector))
  (CallFunction|UpdateAnimation)
  (Transformation|SetWorldRotation (Variables|Default|GetFlipbook_ROOT) (Math|Rotator|MakeRotator 0.0 (* (Class|KismetMathLibrary|DegAcos (Math|Vector|DotProduct _returnvalue "0, 0,1.000000")) (Math|Float|Sign(Float) (Math|Vector|DotProduct _returnvalue "-1.000000, 0, 0"))) 0.0) false false)
  (CallFunction|UpdateAirControlRatio)
  (CallFunction|UpdateFlipbookFacingDirection))

(event Input|ActionEvents|InputActionJump
  (params (Key :type Key%20Structure :default "AnyKey"))
  (:Pressed
    (Class|CustomPawn|Jump)))

(event Input|AxisEvents|InputAxisMoveForward
  (params (AxisValue :type Float%20%28single-precision%29))
  (if (and (!= AxisValue 0.0) (> (Math|Float|Absolute(Float) (Math|Vector|DotProduct (Transformation|GetActorUpVector) "1.000000, 0, 0")) 0.9))
    (Pawn|Input|AddMovementInput "0.000000, 0,1.000000" (* AxisValue (select (AI|Components|NavMovement|IsMovingonGround (Variables|Default|GetMovementComponent)) 1.0 (Variables|/Script/CustomGravityPlugin.CustomMovementComponent|GetAirControlRatio (Variables|Default|GetMovementComponent)))) false)))

(event Input|AxisEvents|InputAxisTurn
  (params (AxisValue :type Float%20%28single-precision%29))
  (if (and (!= AxisValue 0.0) (< (Math|Float|Absolute(Float) (Math|Vector|DotProduct (Transformation|GetActorUpVector) "1.000000, 0, 0")) 0.1))
    (Pawn|Input|AddMovementInput "1.000000, 0,0.000000" (* AxisValue (select (AI|Components|NavMovement|IsMovingonGround (Variables|Default|GetMovementComponent)) 1.0 (Variables|/Script/CustomGravityPlugin.CustomMovementComponent|GetAirControlRatio (Variables|Default|GetMovementComponent)))) false)))

(fn ConstructionScript)